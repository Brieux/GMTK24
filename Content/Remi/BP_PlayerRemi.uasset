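; BP_PlayerRemi is a player actor that builds itself from modular parts saved in BP_GameInstance.
; BeginPlay shows the mouse cursor and walks the Parts map, using each transform key and class value to spawn a part and attach it to BasicBody.
; Holding E activates every spawned part and releasing it deactivates them.
; Tick applies a constant, frame-rate-dependent world drift and local rotation.
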(event `self.ReceiveBeginPlay`
  (bind _parts (`/Game/Blueprints/BP_GameInstance.Parts` (cast `/Game/Blueprints/BP_GameInstance` (`GameplayStatics.GetGameInstance`) :!pure true)))
  (set `PlayerController.bShowMouseCursor` true (`GameplayStatics.GetPlayerController` 0))
  (bind _keys (`BlueprintMapLibrary.Map_Keys` _parts))
  (bind _values (`BlueprintMapLibrary.Map_Values` _parts))
  (for (_array_element _array_index) _keys
    (`self.AddParts` _array_element (`|GetArrayItem` _values _array_index))))

(event `Key|E`
  (params (Key :type "Key Structure"))
  (:`Pressed`
    (for _array_element (`self.SpawnedParts`)
      (`/Game/Remi/BP_StaticPart.Activation` _array_element)))
  (:`Released`
    (for _array_element_2 (`self.SpawnedParts`)
      (`/Game/Remi/BP_StaticPart.Deactivation` _array_element_2))))

(event `self.ReceiveTick`
  (params (DeltaSeconds :type "Float (single-precision)"))
  (`self.K2_AddActorWorldOffset` (0.0 0.2 0.0))
  (`self.K2_AddActorLocalRotation` (struct :`Yaw` 0.2)))

(fn `AddParts`
  (params (RelativeTransform :type "Transform Structure") (PartToSpawn :type "/Game/Remi/BP_StaticPart Class Reference"))
  (bind _returnvalue (`|SpawnActorFromClass` PartToSpawn (`KismetMathLibrary.MakeRelativeTransform` (`SceneComponent.K2_GetComponentToWorld` (`self.BasicBody`)) RelativeTransform) "AlwaysSpawn" "MultiplyWithRoot" null null))
  (`/Game/Remi/BP_StaticPart.AttachParts` _returnvalue (`self.BasicBody`))
  (`KismetArrayLibrary.Array_Add` (`self.SpawnedParts`) _returnvalue))

(fn `UserConstructionScript`)