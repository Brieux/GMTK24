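; BP_StaticPart_Aim is an aiming part whose mesh turns toward the point under the mouse cursor, with a stubbed firing action.
; Tick traces the cursor on the Visibility channel and eases the mesh toward the impact point at RotationInterpSpeed.
; BeginPlay creates a paused looping timer at FireRate, which Activation resumes and Deactivation pauses alongside parent logic.
; The Firing event only prints a debug string.
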(event `self.ReceiveTick`
  (params (DeltaSeconds :type "Float (single-precision)"))
  (bind _staticmesh (`self.StaticMesh`))
  (`parent.ReceiveTick` DeltaSeconds)
  (`SceneComponent.K2_SetWorldRotation` (`self.StaticMesh`) (`KismetMathLibrary.RInterpTo` (`SceneComponent.K2_GetComponentRotation` _staticmesh) (`KismetMathLibrary.FindLookAtRotation` (`SceneComponent.K2_GetComponentLocation` _staticmesh) (`.ImpactPoint` (`GameplayStatics.BreakHitResult` (`PlayerController.GetHitResultUnderCursorByChannel` (`GameplayStatics.GetPlayerController` 0) "TraceTypeQuery1" true)))) DeltaSeconds (`self.RotationInterpSpeed`)) false true))

(event `self.ReceiveBeginPlay`
  (bind _returnvalue (`KismetSystemLibrary.K2_SetTimerDelegate` (`|CreateDelegate` :!event `Firing`) (`self.FireRate`) true true))
  (bind _output_get (set `self.FireHandler` _returnvalue))
  (`KismetSystemLibrary.K2_PauseTimerHandle` _output_get))

(event `Firing`
  (`KismetSystemLibrary.PrintString` "Hello"))

(event `self.Activation`
  (`parent.Activation`)
  (`KismetSystemLibrary.K2_UnPauseTimerHandle` (`self.FireHandler`)))

(event `self.Deactivation`
  (`parent.Deactivation`)
  (`KismetSystemLibrary.K2_PauseTimerHandle` (`self.FireHandler`)))

(fn `UserConstructionScript`
  (`parent.UserConstructionScript`))