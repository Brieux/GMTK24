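; Rotating physics part that spins its main mesh while its part state is Activate.
; On attach, it simulates physics on two extra meshes, chains them to the main mesh with physics constraints, and caches the main constraint's first component.
; Tick applies mass-independent torque around that component's right vector, scaled by RotationSpeed and delta time.
; It also prints the part state every frame for debugging.
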(event `self.ReceiveTick`
  (params (DeltaSeconds :type "Float (single-precision)"))
  (`parent.ReceiveTick` DeltaSeconds)
  (`KismetSystemLibrary.PrintString` (`|GetEnumeratorNameAsString` (`self.PartState`)) true true (struct :`G` 0.66 :`B` 1.0 :`A` 1.0) 0.0)
  (switch `/Game/Remi/EPartState` (`self.PartState`)
    (:`NewEnumerator2`
      (`PrimitiveComponent.AddTorqueInDegrees` (`self.StaticMesh`) (* (`SceneComponent.GetRightVector` (`self.ParentConstraint`)) (* DeltaSeconds (`self.RotationSpeed`))) "None" true))))

(fn `AttachParts`
  (params (ParentToAttachTo :type "PrimitiveComponent Object Reference"))
  (`parent.AttachParts` ParentToAttachTo)
  (`PrimitiveComponent.SetSimulatePhysics` (`self.StaticMesh1`) true)
  (`PrimitiveComponent.SetSimulatePhysics` (`self.StaticMesh2`) true)
  (`PhysicsConstraintComponent.SetConstrainedComponents` (`self.PhysicsConstraint1`) (`self.StaticMesh`) "None" (`self.StaticMesh1`) "None")
  (`PhysicsConstraintComponent.SetConstrainedComponents` (`self.PhysicsConstraint2`) (`self.StaticMesh1`) "None" (`self.StaticMesh2`) "None")
  (bind _outcomponent1 (`PhysicsConstraintComponent.GetConstrainedComponents` (`self.PhysicsConstraint`)))
  (set `self.ParentConstraint` _outcomponent1))

(fn `UserConstructionScript`
  (`parent.UserConstructionScript`))