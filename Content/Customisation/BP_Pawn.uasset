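; Player pawn for the Gundam customisation screen, with a fixed level camera, a mouse cursor and the UI_Custom widget.
; A spawned part follows the cursor each tick via an object trace, aligned to the surface normal and flagging when it is over BP_Gundam.
; On click release it attaches to the Gundam's body and is recorded in PartsPrebuild, or is destroyed if off the robot.
; Right-click input rotates the Gundam, and ResetRotation restores its default facing.
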(event `DestroyPart`
  (set `self.HasSelectedItem` false)
  (`self.K2_DestroyActor` (`self.SpawnedPart`)))

(event `SpawnPart`
  (params (Class :type "/Game/Remi/BP_StaticPart Class Reference"))
  (bind _returnvalue (`|SpawnActorFromClass` Class (`KismetMathLibrary.MakeTransform` (0.0 0.0 0.0)) "Undefined" "MultiplyWithRoot" null null))
  (set `self.SpawnedPart` _returnvalue))

(event `self.ReceiveBeginPlay`
  (bind _returnvalue (`GameplayStatics.GetPlayerController` 0))
  (bind _returnvalue_2 (`GameplayStatics.GetActorOfClass` "/Script/Engine.CameraActor"))
  (bind _output_get (set `self.Cam_Ref` _returnvalue_2))
  (`/Engine/EditorBlueprintResources/StandardMacros.IsValid` _output_get
    (:`Is Valid`
      (`PlayerController.SetViewTargetWithBlend` _returnvalue _returnvalue_2 0.0 "VTBlend_Linear" 0.0 false)
      (set `PlayerController.bShowMouseCursor` true _returnvalue)
      (`EnhancedInputSubsystemInterface.AddMappingContext` (pcsubsystem `EnhancedInputLocalPlayerSubsystem` (`GameplayStatics.GetPlayerController` 0)) "/Game/Customisation/IMC_Actions.IMC_Actions" 0 (struct))
      (bind _returnvalue_3 (`GameplayStatics.GetActorOfClass` "/Game/Customisation/BP_Gundam.BP_Gundam_C"))
      (set `self.Gundam_Ref` _returnvalue_3))))

(event `EnhancedInput|/Game/Customisation/IA_Click`
  (params (ActionValue :type Boolean) (ElapsedSeconds :type "Float (double-precision)") (TriggeredSeconds :type "Float (double-precision)") (InputAction :type "InputAction Object Reference" :default "/Game/Customisation/IA_Click.IA_Click"))
  (bind _hasselecteditem (`self.HasSelectedItem`))
  (bind _onrobot (`self.OnRobot`))
  (:`Completed`
    (if (and _hasselecteditem _onrobot)
      (`/Game/Remi/BP_StaticPart.AttachParts` (`self.SpawnedPart`) (`/Game/Customisation/BP_Gundam.BasicBody` (`self.Gundam_Ref`)))
      (set `self.HasSelectedItem` false)
      (`KismetArrayLibrary.Array_Add` (`self.PartsPrebuild`) (`self.SpawnedPart`))
      (elif (and _hasselecteditem (not _onrobot))
        (`self.DestroyPart`)))))

(event `self.ReceivePossessed`
  (params (NewController :type "Controller Object Reference"))
  (bind _returnvalue (`|CreateWidget` "/Game/Customisation/UI_Custom.UI_Custom_C"))
  (bind _output_get (set `self.UI_Ref` _returnvalue))
  (`UserWidget.AddToViewport` _output_get 0))

(event `EnhancedInput|/Game/Customisation/IA_RightClick`
  (params (ActionValue :type Boolean) (ElapsedSeconds :type "Float (double-precision)") (TriggeredSeconds :type "Float (double-precision)") (InputAction :type "InputAction Object Reference" :default "/Game/Customisation/IA_RightClick.IA_RightClick"))
  (bind (_returnvalue_x _returnvalue_y) (`KismetMathLibrary.BreakVector2D` (`|GetInputActionValue`)))
  (bind _rotationfactor (`self.RotationFactor`))
  (:`Triggered`
    (`self.K2_AddActorWorldRotation` (`self.Gundam_Ref`) (`KismetMathLibrary.MakeRotator` 0.0 (* _rotationfactor _returnvalue_y) (* _returnvalue_x _rotationfactor)) false false)))

(event `ResetRotation`
  (`self.K2_SetActorRotation` (`self.Gundam_Ref`) (struct :`Yaw` 146.428814) false))

(event `self.ReceiveTick`
  (params (DeltaSeconds :type "Float (single-precision)"))
  (bind _spawnedpart (`self.SpawnedPart`))
  (bind _hitresult (`PlayerController.GetHitResultUnderCursorForObjects` (`GameplayStatics.GetPlayerController` 0) (`|MakeArray` "ObjectTypeQuery3" :!type "EObjectTypeQuery Enum") true))
  (if (`self.HasSelectedItem`)
    (`self.K2_SetActorLocation` _spawnedpart (`KismetMathLibrary.SelectVector` (`.Location` (`GameplayStatics.BreakHitResult` _hitresult)) (`.TraceEnd` (`GameplayStatics.BreakHitResult` _hitresult)) (`GameplayStatics.BreakHitResult` _hitresult)) false false)
    (`self.K2_SetActorRotation` _spawnedpart (`KismetMathLibrary.Conv_VectorToRotator` (`.Normal` (`GameplayStatics.BreakHitResult` _hitresult))) false)
    (cast `/Game/Customisation/BP_Gundam` (`.HitActor` (`GameplayStatics.BreakHitResult` _hitresult))
      (:`then`
        (set `self.OnRobot` true))
      (:`CastFailed`
        (set `self.OnRobot` false)))))

(event `GoPlay`
  (`Widget.RemoveFromParent` (`self.UI_Ref`)))

(fn `UserConstructionScript`)